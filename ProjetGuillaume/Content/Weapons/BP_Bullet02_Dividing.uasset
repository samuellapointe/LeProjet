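; BP_Bullet02_Dividing is a projectile that splits into a cluster of smaller bullets about one second after it begins ticking.
; A Delay on Tick leads to disabling collision, destroying the actor, then spawning ten half-scale BP_Bullet03_miniBullets at random points in a surrounding box.
; Each receives a local-space velocity built from its world offset back toward the centre plus a Z boost; the parent's captured velocity is unused.
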(event `self.ReceiveTick`
  (params (DeltaSeconds :type "Float (single-precision)"))
  (`KismetSystemLibrary.Delay` 1.0)
  (bind _returnvalue (`PrimitiveComponent.GetPhysicsLinearVelocity` (`self.CollisionComponent`) "None"))
  (set `self.NewVar_0_0` _returnvalue)
  (`PrimitiveComponent.SetCollisionEnabled` (`self.CollisionComponent`) "NoCollision")
  (`self.K2_DestroyActor`)
  (for _ (range 10)
    (bind _returnvalue_2 (`|SpawnActorFromClass` "/Game/Weapons/BP_Bullet03_miniBullets.BP_Bullet03_miniBullets_C" (`KismetMathLibrary.MakeTransform` (`KismetMathLibrary.RandomPointInBoundingBox` (`self.K2_GetActorLocation`) (`KismetMathLibrary.MakeVector` 200.0 200.0 200.0)) (`self.K2_GetActorRotation`) (0.5 0.5 0.5)) "AdjustIfPossibleButAlwaysSpawn" "OverrideRootScale"))
    (`ProjectileMovementComponent.SetVelocityInLocalSpace` (`/Game/Weapons/BP_Bullet01_Master.Projectile` _returnvalue_2) (+ (* (- (`self.K2_GetActorLocation`) (`SceneComponent.K2_GetComponentLocation` (`/Game/Weapons/BP_Bullet01_Master.CollisionComponent` _returnvalue_2))) 5.0) (0.0 0.0 500.0)))))

(fn `UserConstructionScript`
  (`parent.UserConstructionScript`))