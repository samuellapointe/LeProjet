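; Teleport projectile weapon that moves its owning player to where it lands.
; On hit, a server event searches the hit object's display name for "ground"; a match triggers an all-clients event that teleports the player and plays a sound.
; Both outcomes end in the inherited explosion.
; Tick runs the parent logic and zeroes Wind, while hit and construction retain debug prints.
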(event `self.ReceiveTick`
  (params (DeltaSeconds :type "Float (single-precision)"))
  (`parent.ReceiveTick` 0.0)
  (set `self.Wind` (0.0 0.0 0.0)))

(event `self.ReceiveHit`
  (params (MyComp :type "PrimitiveComponent Object Reference") (Other :type "Actor Object Reference") (OtherComp :type "PrimitiveComponent Object Reference") (bSelfMoved :type Boolean) (HitLocation :type "Vector Structure") (HitNormal :type "Vector Structure") (NormalImpulse :type "Vector Structure") (Hit :type "HitResult Structure (by ref)"))
  ;[1 1 1] Handle Hit
  (`self.REP_Server_HandleHit` Other HitLocation)
  (`KismetSystemLibrary.PrintString` "Hello"))

(event `REP_All_Teleport`
  (params (Player :type "/Game/Characters/GunnerCharacter Object Reference") (Location :type "Vector Structure"))
  ;[1 1 1] Handle Hit
  (`/Game/Characters/GunnerCharacter.Teleport` Player Location)
  (`GameplayStatics.PlaySoundAtLocation` "/Game/Sounds/Animals/S_Martian_woouwoouwoou.S_Martian_woouwoouwoou" Location)
  (`self.REP_All_Explode` :!label _label))

(event `REP_Server_HandleHit`
  (params (Other :type "Actor Object Reference") (`Hit Location` :type "Vector Structure"))
  ;[1 1 1] Handle Hit
  (if (!= (`KismetStringLibrary.FindSubstring` (`KismetSystemLibrary.GetDisplayName` Other) "ground" false false 0) -1)
    (`self.REP_All_Teleport` (`self.MyPlayer`) `Hit Location`)
    (else
      (goto _label))))

(fn `UserConstructionScript`
  (`parent.UserConstructionScript`)
  (`KismetSystemLibrary.PrintString` "WEEEHello"))