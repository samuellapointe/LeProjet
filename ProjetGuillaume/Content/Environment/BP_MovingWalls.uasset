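; BP_MovingWalls is an environment actor that slides along the world X axis according to a boolean, NewVar0, which this graph only reads.
; BeginPlay stores the starting location, and Tick plays or reverses the Movement timeline based on that flag.
; Timeline updates set X to Translation times Distance as an absolute value, keeping the starting Y and Z, without sweeping.
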(event `self.ReceiveBeginPlay`
  (set `self.Starting location` (`self.K2_GetActorLocation`)))

(event `self.ReceiveBeginPlay`)

(event `self.ReceiveActorBeginOverlap`
  (params (OtherActor :type "Actor Object Reference")))

(event `self.ReceiveTick`
  (params (DeltaSeconds :type "Float (single-precision)"))
  (if (`self.NewVar_0`)
    (bind (_direction _translation) (`Timeline|Movement` :!label _label)
      (:`Update`
        (`self.K2_SetActorLocation` (`KismetMathLibrary.MakeVector` (* _translation (`self.Distance`)) (.y (`self.Starting location`)) (.z (`self.Starting location`))))))
    (else
      (goto _label :!via `Reverse`))))

(fn `UserConstructionScript`)