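; Windmill actor with four child-actor wings (BP_Mill_Wing) that spin on the roll axis until each one is fractured.
; The construction script applies a starting roll offset to the wings and builds the per-tick rotation step from RotationSpeed.
; Each Tick, RotateOnServer advances the stored rotation of intact wings, then all four are set to their stored rotations.
; The step is not scaled by delta time, so spin speed follows frame rate.
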(event `RotateOnServer`
  ;[1 1 1] Appliquer une rotation aux ailes qui n'ont pas été détruites
  (`|ExecutionSequence`
    (:`then_0`
      (bind _asbp_mill_wing (cast `/Game/Environment/BP_Mill_Wing` (`ChildActorComponent.ChildActor` (`self.Wing0`))))
      (if (not (`/Game/Environment/BP_Mill_Wing.fractured` _asbp_mill_wing))
        (set `self.RotationWing_0` (`KismetMathLibrary.ComposeRotators` (`SceneComponent.RelativeRotation` (`self.Wing0`)) (`self.RotationSpeed_rot`)))))
    (:`then_1`
      (bind _asbp_mill_wing_2 (cast `/Game/Environment/BP_Mill_Wing` (`ChildActorComponent.ChildActor` (`self.Wing1`))))
      (if (not (`/Game/Environment/BP_Mill_Wing.fractured` _asbp_mill_wing_2))
        (set `self.RotationWing_1` (`KismetMathLibrary.ComposeRotators` (`SceneComponent.RelativeRotation` (`self.Wing1`)) (`self.RotationSpeed_rot`)))))
    (:`then_2`
      (bind _asbp_mill_wing_3 (cast `/Game/Environment/BP_Mill_Wing` (`ChildActorComponent.ChildActor` (`self.Wing2`))))
      (if (not (`/Game/Environment/BP_Mill_Wing.fractured` _asbp_mill_wing_3))
        (set `self.RotationWing_2` (`KismetMathLibrary.ComposeRotators` (`SceneComponent.RelativeRotation` (`self.Wing2`)) (`self.RotationSpeed_rot`)))))
    (:`then_3`
      (bind _asbp_mill_wing_4 (cast `/Game/Environment/BP_Mill_Wing` (`ChildActorComponent.ChildActor` (`self.Wing3`))))
      (if (not (`/Game/Environment/BP_Mill_Wing.fractured` _asbp_mill_wing_4))
        (set `self.RotationWing_3` (`KismetMathLibrary.ComposeRotators` (`SceneComponent.RelativeRotation` (`self.Wing3`)) (`self.RotationSpeed_rot`)))))))

(event `self.ReceiveTick`
  (params (DeltaSeconds :type "Float (single-precision)"))
  ;[1 1 1] Appliquer une rotation aux ailes qui n'ont pas été détruites
  (`self.RotateOnServer`)
  (`|ExecutionSequence`
    (:`then_0`
      (`SceneComponent.K2_SetRelativeRotation` (`self.Wing0`) (`self.RotationWing_0`) false false))
    (:`then_1`
      (`SceneComponent.K2_SetRelativeRotation` (`self.Wing1`) (`self.RotationWing_1`) false false))
    (:`then_2`
      (`SceneComponent.K2_SetRelativeRotation` (`self.Wing2`) (`self.RotationWing_2`) false false))
    (:`then_3`
      (`SceneComponent.K2_SetRelativeRotation` (`self.Wing3`) (`self.RotationWing_3`) false false))))

(fn `UserConstructionScript`
  (`SceneComponent.K2_SetWorldRotation` (`self.Wing0`) (`KismetMathLibrary.MakeRotator` (+ (`self.RotationOffset`) (.roll (`SceneComponent.K2_GetComponentRotation` (`self.Wing0`)))) (.pitch (`SceneComponent.K2_GetComponentRotation` (`self.Wing0`))) (.yaw (`SceneComponent.K2_GetComponentRotation` (`self.Wing0`)))) false false)
  (`SceneComponent.K2_SetWorldRotation` (`self.Wing1`) (`KismetMathLibrary.MakeRotator` (+ (`self.RotationOffset`) (.roll (`SceneComponent.K2_GetComponentRotation` (`self.Wing1`)))) (.pitch (`SceneComponent.K2_GetComponentRotation` (`self.Wing1`))) (.yaw (`SceneComponent.K2_GetComponentRotation` (`self.Wing1`)))) false false)
  (`SceneComponent.K2_SetWorldRotation` (`self.Wing2`) (`KismetMathLibrary.MakeRotator` (+ (`self.RotationOffset`) (.roll (`SceneComponent.K2_GetComponentRotation` (`self.Wing2`)))) (.pitch (`SceneComponent.K2_GetComponentRotation` (`self.Wing2`))) (.yaw (`SceneComponent.K2_GetComponentRotation` (`self.Wing2`)))) false false)
  (`SceneComponent.K2_SetWorldRotation` (`self.Wing3`) (`KismetMathLibrary.MakeRotator` (+ (`self.RotationOffset`) (.roll (`SceneComponent.K2_GetComponentRotation` (`self.Wing3`)))) (.pitch (`SceneComponent.K2_GetComponentRotation` (`self.Wing3`))) (.yaw (`SceneComponent.K2_GetComponentRotation` (`self.Wing3`)))) false false)
  (set `self.RotationSpeed_rot` (`KismetMathLibrary.MakeRotator` (`self.RotationSpeed`))))