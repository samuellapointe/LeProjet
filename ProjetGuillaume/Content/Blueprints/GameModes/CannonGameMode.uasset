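; CannonGameMode is a game mode that gives each joining player their own cannon.
; On PostLogin it takes the first entry from AvailableSpawnLocations and removes it, so no spawn point is reused.
; It spawns a GunnerCharacter there, owned by the new player, and has that player possess it.
; The array is not checked for being empty, and the construction script only prints a debug string.
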(event EventPostLogin
  (params (NewPlayer :type Player%20Controller%20Object%20Reference))
  (Variables|Default|SetnewPlayer NewPlayer) ; Set as variable for reutilisation
  (bind _newparam (CallFunction|GetNewSpawnLocation)) ; Get an unused spawn location
  (bind _returnvalue (Game|SpawnActorfromClass "/Game/Blueprints/Players/GunnerCharacter.GunnerCharacter_C" _newparam "Undefined" (Variables|Default|GetnewPlayer) 0)) ; Spawn a cannon there
  (Pawn|Possess (Variables|Default|GetnewPlayer) _returnvalue) ; And put the player on the seat
)

(fn ConstructionScript
  (Development|PrintString "Construction CannonGameMode"))

(fn GetNewSpawnLocation
  (LocalVariables|Setlocation (Utilities|Array|Get(acopy) (Variables|Default|GetAvailableSpawnLocations)))
  (Utilities|Array|RemoveIndex (Variables|Default|GetAvailableSpawnLocations)) ; Remove it (don't use the same location twice)
  (return (LocalVariables|Getlocation)))