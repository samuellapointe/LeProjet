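; BP_Zipplin is an airship-style actor that crashes in flames when its capsule is hit.
; The hit calls a Multicast event that activates explosion, fire and electricity effects and plays a Crash timeline.
; The timeline's curves set the root's absolute world height and yaw, keeping X and Y.
; When it finishes, the explosion is scaled up and activated again for the final blast.
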(event `self.Capsule.OnComponentHit`
  (params (OtherActor :type "Actor Object Reference") (OtherComp :type "PrimitiveComponent Object Reference") (NormalImpulse :type "Vector Structure") (Hit :type "HitResult Structure (by ref)"))
  (`self.Multicast`))

(event `Multicast`
  (bind _explosion (`self.explosion`))
  (`ActorComponent.Activate` (`self.explosion`) false)
  (`ActorComponent.Activate` (`self.BigFire`) false)
  (`ActorComponent.Activate` (`self.Electricity`) false)
  (bind (_direction _height _rotation) (`Timeline|Crash`)
    (:`Update`
      (`SceneComponent.K2_SetWorldLocation` (`self.DefaultSceneRoot`) (`KismetMathLibrary.MakeVector` (.x (`self.K2_GetActorLocation`)) (.y (`self.K2_GetActorLocation`)) _height) false false)
      (`SceneComponent.K2_SetWorldRotation` (`self.DefaultSceneRoot`) (`KismetMathLibrary.MakeRotator` 0.0 0.0 _rotation) false false))
    (:`Finished`
      (`SceneComponent.SetWorldScale3D` _explosion (20.0 20.0 20.0))
      (`ActorComponent.Activate` _explosion false))))

(fn `UserConstructionScript`)